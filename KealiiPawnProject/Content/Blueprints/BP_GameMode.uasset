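; BP_GameMode is a game mode Blueprint that respawns the player's pawn whenever it is destroyed.
; On BeginPlay it binds to the current BP_PlayerPawn's OnDestroyed event.
; After a half-second delay, the handler spawns a new pawn at the SpawnTransform variable and has player controller 0 possess it.
; It then calls Respawn to bind to the new pawn, so the cycle repeats.
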(event Custom|Respawn
  (bind _asbp_player_pawn (Utilities|Casting|CastToBP_PlayerPawn (Game|Player|GetPlayerPawn 0)))
  (Game|BindEventtoOnDestroyed _asbp_player_pawn (delegate Custom|OnDestoryed_Event)))

(event Custom|OnDestoryed_Event
  (params (DestroyedActor :type Actor%20Object%20Reference))
  (Utilities|FlowControl|Delay 0.5)
  (bind _returnvalue (Game|SpawnActorfromClass "/Game/Blueprints/BP_PlayerPawn.BP_PlayerPawn_C" (Variables|Default|GetSpawn%20Transform) "AdjustIfPossibleButAlwaysSpawn" 0 0))
  (Pawn|Possess (Game|GetPlayerController 0) _returnvalue)
  (CallFunction|Respawn))

(event EventBeginPlay
  (bind _asbp_player_pawn (Utilities|Casting|CastToBP_PlayerPawn (Game|Player|GetPlayerPawn 0)))
  (Game|BindEventtoOnDestroyed _asbp_player_pawn (delegate Custom|OnDestoryed_Event)))

(event EventTick
  (params (DeltaSeconds :type Float%20%28single-precision%29)))

(fn ConstructionScript)