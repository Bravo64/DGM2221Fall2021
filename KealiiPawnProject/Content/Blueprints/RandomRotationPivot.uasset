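; Pivot actor that spins on a single axis at a randomly changing speed.
; On BeginPlay it starts SetNewSpeed, which picks a rate between MinimumSpeed and MaximumSpeed and writes it to the RotatingMovement component.
; The event re-calls itself after a random delay of a few seconds, so speed changes in abrupt steps without using Tick.
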(event Custom|SetNewSpeed
  (bind _output_get (Variables|Default|SetRotationRate (Math|Random|RandomFloatinRange (Variables|Default|GetMinimumSpeed) (Variables|Default|GetMaximumSpeed))))
  (Variables|/Script/Engine.RotatingMovementComponent|SetRotationRate (Variables|Default|GetRotatingMovement) (Math|Rotator|MakeRotator 0.0 0.0 _output_get))
  (Utilities|FlowControl|Delay (Math|Random|RandomFloatinRange 2.0 4.0))
  (CallFunction|SetNewSpeed))

(event EventBeginPlay
  (CallFunction|SetNewSpeed))

(event Collision|EventActorBeginOverlap
  (params (OtherActor :type Actor%20Object%20Reference)))

(event EventTick
  (params (DeltaSeconds :type Float%20%28single-precision%29)))

(fn ConstructionScript)