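; BP_PlayerPawn is a player pawn that moves by rolling its RollingStone component with physics.
; Forward/backward and right/left axis inputs apply torque around Y and X, scaled by TorqueStrength and applied as an acceleration change so mass is ignored.
; A K key debug-style kill destroys the pawn and snaps the camera to a held fade-out, ending in a short delay with nothing after it.
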(event EventBeginPlay)

(event Collision|EventActorBeginOverlap
  (params (OtherActor :type Actor%20Object%20Reference)))

(event EventTick
  (params (DeltaSeconds :type Float%20%28single-precision%29)))

(event Input|AxisEvents|InputAxisMoveForwards/Backwards
  (params (AxisValue :type Float%20%28single-precision%29))
  (Class|PrimitiveComponent|AddTorqueinRadians (Variables|Default|GetRollingStone) (Math|Vector|MakeVector 0.0 (* AxisValue (Variables|Default|GetTorqueStrength)) 0.0) "None" true))

(event Input|AxisEvents|InputAxisMoveRight/Left
  (params (AxisValue :type Float%20%28single-precision%29))
  (Class|PrimitiveComponent|AddTorqueinRadians (Variables|Default|GetRollingStone) (Math|Vector|MakeVector (* AxisValue (Variables|Default|GetTorqueStrength)) 0.0 0.0) "None" true))

(event Input|KeyboardEvents|K
  (params (Key :type Key%20Structure :default "None"))
  ;[1 1 1] Keyboard Kill Actor
  (:Pressed
    (Actor|DestroyActor)
    (CameraFades|StartCameraFade :self (Game|GetPlayerCameraManager 0) :ToAlpha 1.0 :Duration 0.01 :bHoldWhenFinished true)
    (Utilities|FlowControl|Delay 0.01)))

(fn ConstructionScript)